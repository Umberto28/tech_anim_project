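; BP_HealthPickUp is a health pickup that heals a BP_TACharacter overlapping its box, but only when that character is below max health.
; Healing is applied by calling the character's TakeDamage with the negated Heal value.
; It then tells the BP_HealthSpawn found through GetActorOfClass on BeginPlay to respawn a pickup, and destroys itself.
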(event OnComponentBeginOverlap(Box)
  (params (OverlappedComponent :type Primitive%20Component%20Object%20Reference) (OtherActor :type Actor%20Object%20Reference) (OtherComp :type Primitive%20Component%20Object%20Reference) (OtherBodyIndex :type Integer) (bFromSweep :type Boolean) (SweepResult :type Hit%20Result%20Structure%20%28by%20ref%29))
  (bind _asbp_tacharacter (Utilities|Casting|CastToBP_TACharacter OtherActor))
  (if (CallFunction|HealthCheck _asbp_tacharacter)
    (Default|TakeDamage _asbp_tacharacter (Math|Conversions|ToFloat(Integer) (* (Variables|Default|GetHeal) -1)))
    (Default|RespawnHealthPickUp (Variables|Default|GetRefToHealthSpawn))
    (Actor|DestroyActor)))

(event EventBeginPlay
  (bind _returnvalue (Actor|GetActorOfClass "/Game/Master/Blueprints/BP_HealthSpawn.BP_HealthSpawn_C"))
  (Variables|Default|SetRefToHealthSpawn _returnvalue))

(fn ConstructionScript)

(fn HealthCheck
  (params (self2 :type BP%20TA%20Character%20Object%20Reference))
  (return (> (Variables|/Game/Master/Characters/MainCharacter/Blueprints/BP_TACharacter.BP_TACharacter_C|GetMaxHealth self2) (Variables|/Game/Master/Characters/MainCharacter/Blueprints/BP_TACharacter.BP_TACharacter_C|GetHealth self2))))