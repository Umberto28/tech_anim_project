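; Game mode that runs endless, escalating enemy waves from BP_AI_Spawn actors in the level.
; On BeginPlay it caches the player character and all spawners, then starts the first wave.
; Each wave raises the enemy count by one and calls EnemiesSpawn on a randomly picked spawner per enemy.
; EnemyDeath decrements the alive count and starts the next wave when it reaches zero.
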(event Custom|EnemyDeath
  (bind _enemiesalive (Variables|Default|GetEnemiesAlive))
  (Math|Integer|DecrementInt _enemiesalive
    (:%20%20
      (if (== _enemiesalive 0)
        (CallFunction|RespawnEnemies)))))

(event Custom|RespawnEnemies
  (CallFunction|EnemyCounter)
  (for _index (range 1 (Variables|Default|GetSpawned%20Enemy))
    (Default|EnemiesSpawn (.OutItem (Utilities|Array|Random (Variables|Default|GetSpawners))))
    (Math|Integer|IncrementInt (Variables|Default|GetEnemiesAlive))))

(event EventBeginPlay
  (bind _asbp_tacharacter (Utilities|Casting|CastToBP_TACharacter (Game|GetPlayerCharacter 0)))
  (Variables|Default|SetRefToCharacter _asbp_tacharacter)
  (bind _outactors (Actor|GetAllActorsOfClass "/Game/Master/Characters/AI/BP_AI_Spawn.BP_AI_Spawn_C"))
  (Variables|Default|SetSpawners _outactors)
  (CallFunction|RespawnEnemies))

(fn ConstructionScript)

(fn EnemyCounter
  (Math|Integer|IncrementInt (Variables|Default|GetSpawned%20Enemy)))