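; Game mode for a wave-based local multiplayer game that runs enemy rounds and sets up each player's camera and HUD.
; On BeginPlay it creates extra local players from the game instance's player count, giving each a camera handler tied to the level's camera spline, then adds a HUD per controller.
; Each round spawns one more enemy from random AI spawn points, and the next starts when all are dead.
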(event Custom|EnemyDeath
  (bind _enemiesalive (Variables|Default|GetEnemiesAlive))
  (Math|Integer|DecrementInt _enemiesalive
    (:%20%20
      (if (== _enemiesalive 0)
        (CallFunction|RespawnEnemies)))))

(event Custom|RespawnEnemies
  (Math|Integer|IncrementInt (Variables|Default|GetRoundCounter)
    (:%20%20
      (CallFunction|EnemyCounter)
      (for _index (range 1 (Variables|Default|GetSpawned%20Enemy))
        (Default|EnemiesSpawn (.OutItem (Utilities|Array|Random (Variables|Default|GetSpawners))))
        (Math|Integer|IncrementInt (Variables|Default|GetEnemiesAlive))))))

(event EventBeginPlay
  (bind _outactors (Actor|GetAllActorsOfClass "/Game/Master/Characters/AI/BP_AI_Spawn.BP_AI_Spawn_C"))
  (Variables|Default|SetSpawners _outactors)
  (CallFunction|RespawnEnemies)
  (bind (_returnvalue _playernumber) (|CheckIfMultiplayer))
  (if _returnvalue
    (for _index (range 2 _playernumber)
      ;[1 1 1] Handling Multiplayer Camera
      (bind _returnvalue_2 (Class|GameplayStatics|CreatePlayer -1))
      (Development|PrintString "spawn player")
      (bind _returnvalue_3 (Actor|GetActorOfClass "/Game/Master/Characters/MainCharacter/Blueprints/BP_CameraSpline.BP_CameraSpline_C"))
      (bind _asbp_tacharacter (Utilities|Casting|CastToBP_TACharacter (Pawn|GetControlledPawn _returnvalue_2)))
      (Game|SpawnActorfromClass "/Game/Master/Blueprints/Props/BP_CameraHandler.BP_CameraHandler_C" (Variables|Default|GetHandlerTransform) "Undefined" "MultiplyWithRoot" 0 _returnvalue_3 5.5e+02 _asbp_tacharacter 0)
      (Variables|/Game/Master/Characters/MainCharacter/Blueprints/BP_TACharacter.BP_TACharacter_C|SetRefToCameraSpline _asbp_tacharacter _returnvalue_3)
      (Transformation|SetActorRotation (Pawn|GetControlledPawn _returnvalue_2) "0.000000,90.000000,0.000000")))
  ;[1 1 1] Adding Player Screen UI
  (bind _outactors_2 (Actor|GetAllActorsOfClass "/Game/Master/Characters/MainCharacter/Blueprints/BP_TAPlayerController.BP_TAPlayerController_C"))
  (for _array_element _outactors_2
    (bind _returnvalue_4 (UserInterface|CreateWidget "/Game/Master/UI/Widgets/WBP_Hud.WBP_Hud_C" _array_element))
    (UserInterface|Viewport|AddtoPlayerScreen _returnvalue_4)))

(fn ConstructionScript)

(fn EnemyCounter
  (Math|Integer|IncrementInt (Variables|Default|GetSpawned%20Enemy)))