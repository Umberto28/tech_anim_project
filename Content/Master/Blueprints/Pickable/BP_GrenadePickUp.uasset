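; Grenade pickup actor that refills a character's grenades to maximum on overlap.
; On mesh overlap with a BP_TACharacter, it checks that the current count is below max before filling it.
; It then tells the BP_GrenadeSpawn actor, found by class lookup at BeginPlay, to respawn the pickup and destroys itself.
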(event OnComponentBeginOverlap(StaticMesh)
  (params (OverlappedComponent :type Primitive%20Component%20Object%20Reference) (OtherActor :type Actor%20Object%20Reference) (OtherComp :type Primitive%20Component%20Object%20Reference) (OtherBodyIndex :type Integer) (bFromSweep :type Boolean) (SweepResult :type Hit%20Result%20Structure%20%28by%20ref%29))
  (bind _asbp_tacharacter (Utilities|Casting|CastToBP_TACharacter OtherActor))
  (if (.ReturnValue (CallFunction|CheckGrenades _asbp_tacharacter))
    (Variables|/Game/Master/Characters/MainCharacter/Blueprints/BP_TACharacter.BP_TACharacter_C|SetCurrGrenades _asbp_tacharacter (.MaxGrenades (CallFunction|CheckGrenades _asbp_tacharacter)))
    (Default|RespawnGrenadePickUp (Variables|Default|GetRefToGrenadeSpawn))
    (Actor|DestroyActor)))

(event EventBeginPlay
  (bind _returnvalue (Actor|GetActorOfClass "/Game/Master/Blueprints/Pickable/BP_GrenadeSpawn.BP_GrenadeSpawn_C"))
  (Variables|Default|SetRefToGrenadeSpawn _returnvalue))

(fn ConstructionScript)

(fn CheckGrenades
  (params (self2 :type BP%20TA%20Character%20Object%20Reference))
  (bind _maxgrenades (Variables|/Game/Master/Characters/MainCharacter/Blueprints/BP_TACharacter.BP_TACharacter_C|GetMaxGrenades self2))
  (return (> _maxgrenades (Variables|/Game/Master/Characters/MainCharacter/Blueprints/BP_TACharacter.BP_TACharacter_C|GetCurrGrenades self2)) _maxgrenades))