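; Spawner actor that places BP_GrenadePickUp actors in the level.
; It spawns one on BeginPlay, and its RespawnGrenadePickUp event spawns another after a five-second delay.
; The SpawnLocation&Rotation graph builds the transform from the Billboard's X and rotation, with random Y and Z.
; It samples a reachable navigation point within SpawnRadius of the Billboard and raises the height by a fixed offset.
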(event Custom|RespawnGrenadePickUp
  (bind (_x _randomy _randomz _rotation) (|SpawnLocation&Rotation))
  (Utilities|FlowControl|Delay 5.0)
  (Game|SpawnActorfromClass "/Game/Master/Blueprints/Pickable/BP_GrenadePickUp.BP_GrenadePickUp_C" (Math|Transform|MakeTransform (Math|Vector|MakeVector _x _randomy _randomz) _rotation "1.000000,1.000000,1.000000") "Undefined" "MultiplyWithRoot" 0 0))

(event EventBeginPlay
  (bind (_x _randomy _randomz _rotation) (|SpawnLocation&Rotation))
  (Game|SpawnActorfromClass "/Game/Master/Blueprints/Pickable/BP_GrenadePickUp.BP_GrenadePickUp_C" (Math|Transform|MakeTransform (Math|Vector|MakeVector _x _randomy _randomz) _rotation "1.000000,1.000000,1.000000") "Undefined" "MultiplyWithRoot" 0 0))

(fn ConstructionScript)