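; Trigger volume prop that raises the BP_CameraSpline actor while the player is inside its box and lowers it on exit.
; BeginPlay caches the spline and player, then derives both target heights from the spline's starting Z plus Distance.
; Box overlaps set GoingUp and enable Tick, which interpolates the spline's Z with VInterpTo.
; Tick disables itself when CheckIfEndedMovement returns true, though that function's height comparisons appear unconnected.
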(event OnComponentBeginOverlap(Box)
  (params (OverlappedComponent :type Primitive%20Component%20Object%20Reference) (OtherActor :type Actor%20Object%20Reference) (OtherComp :type Primitive%20Component%20Object%20Reference) (OtherBodyIndex :type Integer) (bFromSweep :type Boolean) (SweepResult :type Hit%20Result%20Structure%20%28by%20ref%29))
  ;[1 1 1] Trigger to Move Camera Up
  (bind _asbp_tacharacter (Utilities|Casting|CastToBP_TACharacter OtherActor))
  (if (== _asbp_tacharacter (Variables|Default|GetRefToPlayer))
    (Variables|Default|SetGoingUp true)
    (Actor|Tick|SetActorTickEnabled true)))

(event OnComponentEndOverlap(Box)
  (params (OverlappedComponent :type Primitive%20Component%20Object%20Reference) (OtherActor :type Actor%20Object%20Reference) (OtherComp :type Primitive%20Component%20Object%20Reference) (OtherBodyIndex :type Integer))
  ;[1 1 1] Trigger To Move Camera Down
  (bind _asbp_tacharacter (Utilities|Casting|CastToBP_TACharacter OtherActor))
  (if (== _asbp_tacharacter (Variables|Default|GetRefToPlayer))
    (Variables|Default|SetGoingUp false)
    (Actor|Tick|SetActorTickEnabled true)))

(event EventTick
  (params (DeltaSeconds :type Float%20%28single-precision%29))
  (bind (_returnvalue _returnvalue2) (|CheckIfEndedMovement))
  (if (Variables|Default|GetGoingUp)
    (CallFunction|MoveCameraUp)
    (if _returnvalue
      (Actor|Tick|SetActorTickEnabled false :!label _label))
    (else
      (CallFunction|MoveCameraDown)
      (if _returnvalue2
        (goto _label)))))

(event EventBeginPlay
  (Utilities|IsValid (Variables|Default|GetRefToCameraSpline)
    (:Is%20Valid
      _)
    (:Is%20Not%20Valid
      (bind _returnvalue (Actor|GetActorOfClass "/Game/Master/Characters/MainCharacter/Blueprints/BP_CameraSpline.BP_CameraSpline_C"))
      (bind _output_get (Variables|Default|SetRefToCameraSpline _returnvalue))))
  (Utilities|IsValid (Variables|Default|GetRefToPlayer)
    (:Is%20Valid
      _)
    (:Is%20Not%20Valid
      (bind _asbp_tacharacter (Utilities|Casting|CastToBP_TACharacter (Game|GetPlayerCharacter 0)))
      (Variables|Default|SetRefToPlayer _asbp_tacharacter)))
  (|SetCameraZvalues (.z (Transformation|GetActorLocation _output_get))))

(fn ConstructionScript)

(fn MoveCameraUp
  (bind _reftocameraspline (Variables|Default|GetRefToCameraSpline))
  (bind _returnvalue (Transformation|GetActorLocation _reftocameraspline))
  (bind (_x _y) (Math|Vector|BreakVector _returnvalue))
  (Transformation|SetActorLocation _reftocameraspline (Math|Interpolation|VInterpTo _returnvalue (Math|Vector|MakeVector _x _y (Variables|Default|GetTargetZUp)) (Utilities|Time|GetWorldDeltaSeconds) 8.0) false false))

(fn MoveCameraDown
  (bind _reftocameraspline (Variables|Default|GetRefToCameraSpline))
  (bind _returnvalue (Transformation|GetActorLocation _reftocameraspline))
  (bind (_x _y) (Math|Vector|BreakVector _returnvalue))
  (Transformation|SetActorLocation _reftocameraspline (Math|Interpolation|VInterpTo _returnvalue (Math|Vector|MakeVector _x _y (Variables|Default|GetTargetZDown)) (Utilities|Time|GetWorldDeltaSeconds) 8.0) false false))