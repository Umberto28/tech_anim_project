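; BP_AI_Bot is an AI enemy character that takes weapon damage, awards score on death and can jump to destinations.
; BotTakeDamage clamps health and triggers Death at zero.
; Death ragdolls the mesh, ignores two capsule trace channels, adds to the cached player's score, then after a delay notifies BP_TAGameMode and destroys the actor.
; JumpToDestination launches the character along a suggested projectile arc, aimed above the target.
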(event Custom|Death
  (bind _reftoplayer (Variables|Default|GetRefToPlayer))
  (Variables|Default|SetIsDead true)
  (|CollisionAndPhysicsUpdate)
  (Character|Crouch)
  (Variables|/Game/Master/Characters/MainCharacter/Blueprints/BP_TACharacter.BP_TACharacter_C|SetScore _reftoplayer (+ (Variables|/Game/Master/Characters/MainCharacter/Blueprints/BP_TACharacter.BP_TACharacter_C|GetScore _reftoplayer) 100))
  (bind _asbp_tagame_mode (Utilities|Casting|CastToBP_TAGameMode (Game|GetGameMode)))
  (Utilities|FlowControl|Delay 2.6)
  (Default|EnemyDeath _asbp_tagame_mode)
  (Actor|DestroyActor))

(event EventBeginPlay
  (Variables|Default|SetCurrentHealth (Variables|Default|GetMaxHealth))
  (bind _asbp_tacharacter (Utilities|Casting|CastToBP_TACharacter (Game|Player|GetPlayerPawn 0)))
  (Variables|Default|SetRefToPlayer _asbp_tacharacter))

(fn ConstructionScript)

(fn BotTakeDamage
  (params (Weapon%20Damage :type Integer))
  (Variables|Default|SetCurrentHealth (Math|Integer|Clamp(Integer) (- (Variables|Default|GetCurrentHealth) Weapon%20Damage) 0 (Variables|Default|GetMaxHealth)))
  (if (<= (Variables|Default|GetCurrentHealth) 0)
    (CallFunction|Death)))

(fn JumptoDestination
  (params (Destination :type Vector))
  (bind (_x _y _z) (Math|Vector|BreakVector Destination))
  (bind _outlaunchvelocity (Game|SuggestProjectileVelocityCustomArc (Transformation|GetActorLocation) (Math|Vector|MakeVector _x _y (+ _z 1.7e+02)) 0.0 0.5))
  (Character|LaunchCharacter _outlaunchvelocity true true))