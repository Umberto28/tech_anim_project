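; BP_AI_Spawn is a spawner that places BP_AI_Bot enemies in the level, each running BT_AI_Bot.
; EnemiesSpawn spawns one bot using the Billboard's location and rotation, ignoring collision failure.
; GetSpawnXOffset and GetSpawnYOffset supply X and Y, with random-range nodes around the Billboard position bounded by offset variables, while Z stays at the Billboard's height.
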(fn ConstructionScript)

(fn EnemiesSpawn
  (bind _billboard (Variables|Default|GetBillboard))
  (bind _returnvalue (Transformation|GetWorldLocation _billboard))
  (AI|SpawnAIFromClass "/Game/Master/Characters/AI/BP_AI_Bot.BP_AI_Bot_C" "/Game/Master/Characters/AI/BT_AI_Bot.BT_AI_Bot" (Math|Vector|MakeVector (|GetSpawnXOffset (.x _returnvalue) (.x _returnvalue)) (|GetSpawnYOffset (.y _returnvalue) (.y _returnvalue)) (.z _returnvalue)) (Transformation|GetWorldRotation _billboard) true 0)
  (return))