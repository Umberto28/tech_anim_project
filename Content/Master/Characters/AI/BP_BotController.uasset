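; AI controller for BP_AI_Bot that runs BT_AI_Bot on possession and drives the bot's targeting and aim.
; Each tick, outside singleplayer, it retargets the nearest player from living characters, appended to ActorsToCheck without clearing.
; It points the bot's arrow at the target, stores aim pitch, and uses the yaw sign to set Forward and flip the mesh 180 degrees.
; Once the bot dies, it stops movement and disables its tick.
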(event EventTick
  (params (DeltaSeconds :type Float%20%28single-precision%29))
  (bind _reftobot (Variables|Default|GetRefToBot))
  (if (Variables|/Game/Master/Characters/AI/BP_AI_Bot.BP_AI_Bot_C|GetIsDead _reftobot)
    (AI|Navigation|StopMovement)
    (Actor|Tick|SetActorTickEnabled false)
    (else
      (if (Variables|/Game/Master/Characters/AI/BP_AI_Bot.BP_AI_Bot_C|GetIsSingleplayer _reftobot)
        _
        (else
          (CallFunction|FindNearestPlayer)))
      (bind (_aimpitch _aimyaw) (CallFunction|AimLocation))
      (Variables|Default|SetAim%20Pitch _aimpitch)
      (bind _forward_ (CallFunction|TurningBot _aimyaw))
      (Variables|Default|SetForward? _forward_))))

(event EventPossess
  (params (PossessedPawn :type Pawn%20Object%20Reference))
  (bind _asbp_ai_bot (Utilities|Casting|CastToBP_AI_Bot PossessedPawn))
  (Variables|Default|SetRefToBot _asbp_ai_bot)
  (AI|RunBehaviorTree "/Game/Master/Characters/AI/BT_AI_Bot.BT_AI_Bot"))

(fn ConstructionScript)

(fn AimLocation
  (bind _reftobot (Variables|Default|GetRefToBot))
  (bind _returnvalue (Transformation|GetActorLocation _reftobot))
  (bind _reftoplayer (Variables|/Game/Master/Characters/AI/BP_AI_Bot.BP_AI_Bot_C|GetRefToPlayer _reftobot))
  (bind _returnvalue_2 (Transformation|GetActorLocation _reftoplayer))
  (bind _returnvalue_3 (- _returnvalue_2 _returnvalue))
  (bind _returnvalue_4 (Math|Rotator|MakeRotfromX _returnvalue_3))
  (bind (_roll _pitch _yaw) (Math|Rotator|BreakRotator _returnvalue_4))
  (Transformation|SetWorldRotation (Variables|/Game/Master/Characters/AI/BP_AI_Bot.BP_AI_Bot_C|GetArrow1 (Variables|Default|GetRefToBot)) _returnvalue_4 false false)
  (return _pitch _yaw))

(fn TurningBot
  (params (AimYaw :type Float%20%28double-precision%29))
  (bind _reftobot (Variables|Default|GetRefToBot))
  (bind _mesh (Variables|/Script/Engine.Character|GetMesh _reftobot))
  (if (== (/ AimYaw (Math|Float|Absolute(Float) AimYaw)) 1.0)
    (Variables|Default|SetForward? true)
    (Transformation|SetWorldRotation _mesh "0, 0, 0" false false)
    (else
      (Variables|Default|SetForward? false)
      (Transformation|SetWorldRotation _mesh "0.000000,180.000000,0.000000" false false)))
  (return (Variables|Default|GetForward?)))

(fn FindNearestPlayer
  (bind _outactors (Actor|GetAllActorsOfClass "/Game/Master/Characters/MainCharacter/Blueprints/BP_TACharacter.BP_TACharacter_C"))
  (for _array_element _outactors
    (if (not (Variables|/Game/Master/Characters/MainCharacter/Blueprints/BP_TACharacter.BP_TACharacter_C|GetIsDead _array_element))
      (Utilities|Array|Add (Variables|Default|GetActorsToCheck) _array_element)))
  (bind _asbp_tacharacter (Utilities|Casting|CastToBP_TACharacter (.ReturnValue (Actor|FindNearestActor (Transformation|GetActorLocation (Variables|Default|GetRefToBot)) (Variables|Default|GetActorsToCheck)))))
  (Variables|/Game/Master/Characters/AI/BP_AI_Bot.BP_AI_Bot_C|SetRefToPlayer (Variables|Default|GetRefToBot) _asbp_tacharacter))