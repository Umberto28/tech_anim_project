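; Actor component that flashes its owner's skeletal mesh by pulsing material emissive values, as damage feedback.
; On BeginPlay it creates a dynamic material instance from slot 0, also assigns it to slot 1, and caches the original emissive color and multiplier.
; The DamageFlash event alternates between the flash and cached values, with delays, for a configurable number of blinks.
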(event Custom|DamageFlash
  (bind _flashmat (Variables|Default|GetFlashMat))
  (bind _flashmat_2 (Variables|Default|GetFlashMat))
  (for _index (range 1 (Variables|Default|GetFlashOccur))
    ;[1 1 1] Flash Values
    (Rendering|Material|SetVectorParameterValue _flashmat_2 "EmissiveColor" (Variables|Default|GetFlashColor) :!class /Script/Engine.MaterialInstanceDynamic)
    (Rendering|Material|SetScalarParameterValue _flashmat_2 "EmissiveMultiplier" (Variables|Default|GetFlashMult) :!class /Script/Engine.MaterialInstanceDynamic)
    (Utilities|FlowControl|Delay (Variables|Default|GetFlashDuration))
    ;[1 1 1] Return Original Values
    (Rendering|Material|SetVectorParameterValue _flashmat "EmissiveColor" (Variables|Default|GetInitEmissiveColor) :!class /Script/Engine.MaterialInstanceDynamic)
    (Rendering|Material|SetScalarParameterValue _flashmat "EmissiveMultiplier" (Variables|Default|GetInitEmissiveMultiplier) :!class /Script/Engine.MaterialInstanceDynamic)
    (Utilities|FlowControl|Delay (Variables|Default|GetFlashDuration))))

(event EventBeginPlay
  (bind _output_get (Variables|Default|SetRefToOwner (Components|GetOwner)))
  ;[1 1 1] Setup Dynamic Mat Instance
  (Utilities|IsValid (Actor|GetComponentbyClass _output_get "/Script/Engine.SkeletalMeshComponent")
    (:Is%20Valid
      (bind _returnvalue (Rendering|Material|CreateDynamicMaterialInstance (Actor|GetComponentbyClass _output_get "/Script/Engine.SkeletalMeshComponent") 0 0 "None" :!class /Script/Engine.PrimitiveComponent))
      (bind _output_get_2 (Variables|Default|SetFlashMat _returnvalue))
      (Rendering|Material|SetMaterial (Actor|GetComponentbyClass _output_get "/Script/Engine.SkeletalMeshComponent") 1 _output_get_2)
      ;[1 1 1] Get Init Emissive Values
      (bind _returnvalue_2 (Rendering|Material|GetVectorParameterValue _output_get_2 "EmissiveColor" :!class /Script/Engine.MaterialInstanceDynamic))
      (Variables|Default|SetInitEmissiveColor _returnvalue_2)
      (bind _returnvalue_3 (Rendering|Material|GetScalarParameterValue _output_get_2 "EmissiveMultiplier" :!class /Script/Engine.MaterialInstanceDynamic))
      (Variables|Default|SetInitEmissiveMultiplier _returnvalue_3))))