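; Player character that manages health, score and grenade attributes, resetting them and finding the camera spline on BeginPlay.
; TakeDamage applies clamped health changes; positive damage triggers a flash and temporary invincibility by ignoring the capsule's Visibility channel.
; At zero health, Death notifies the player controller, disables some capsule collision responses and flags the character dead.
; CustomMovement moves only along the inverted control-rotation right vector; its forward input is unwired.
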(event Custom|Invincibility
  (Collision|SetCollisionResponsetoChannel (Variables|Collision|GetCapsuleComponent) "ECC_Visibility" "ECR_Ignore")
  (Utilities|FlowControl|Delay (Variables|Default|GetInvincibilityDuration))
  (Collision|SetCollisionResponsetoChannel (Variables|Collision|GetCapsuleComponent) "ECC_Visibility" "ECR_Block"))

(event EventBeginPlay
  (Utilities|IsValid (Variables|Default|GetRefToCameraSpline)
    (:Is%20Valid
      _)
    (:Is%20Not%20Valid
      (bind _returnvalue (Actor|GetActorOfClass "/Game/Master/Characters/MainCharacter/Blueprints/BP_CameraSpline.BP_CameraSpline_C"))
      (Variables|Default|SetRefToCameraSpline _returnvalue)))
  (CallFunction|SetBaseAttribute))

(fn ConstructionScript)

(fn CustomMovement
  (params (ActionValueX :type Float%20%28double-precision%29) (ActionValueY :type Float%20%28double-precision%29))
  (bind _returnvalue (Pawn|GetControlRotation :!class /Script/Engine.Pawn))
  (Pawn|Input|AddMovementInput (* (Math|Vector|GetRightVector (Math|Rotator|MakeRotator (.roll _returnvalue) 0.0 (.yaw _returnvalue))) -1) ActionValueX false))

(fn TakeDamage
  (params (WeaponDamage :type Float%20%28double-precision%29))
  (bind (_clamp _health) (|ClampHealth WeaponDamage))
  (Variables|Default|SetHealth _clamp)
  (if (> WeaponDamage 0.0)
    (Default|DamageFlash (Variables|Default|GetBP_Damage_flash))
    (CallFunction|Invincibility)
    (if (<= _health 0.0)
      (CallFunction|Death))))

(fn Death
  (bind _capsulecomponent (Variables|Collision|GetCapsuleComponent))
  (bind _asbp_taplayer_controller (Utilities|Casting|CastToBP_TAPlayerController (Pawn|GetController)))
  (Default|PlayerDeath _asbp_taplayer_controller)
  (Collision|SetCollisionResponsetoChannel _capsulecomponent "ECC_Pawn" "ECR_Ignore")
  (Collision|SetCollisionResponsetoChannel _capsulecomponent "ECC_GameTraceChannel1" "ECR_Ignore")
  (Variables|Default|SetIsDead true))

(fn SetBaseAttribute
  (Variables|Default|SetHealth (Variables|Default|GetMaxHealth))
  (Variables|Default|SetScore 0)
  (Variables|Default|SetCurrGrenades (Variables|Default|GetMaxGrenades)))