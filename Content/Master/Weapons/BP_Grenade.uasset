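; BP_Grenade is a timed explosive that damages AI bots within its blast volume.
; It detonates three seconds after spawning, or immediately when its capsule overlaps a BP_AI_Bot.
; Detonation applies damage via BotTakeDamage to every bot overlapping the Explosion component, then destroys the grenade.
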(event OnComponentBeginOverlap(capsule_0)
  (params (OverlappedComponent :type Primitive%20Component%20Object%20Reference) (OtherActor :type Actor%20Object%20Reference) (OtherComp :type Primitive%20Component%20Object%20Reference) (OtherBodyIndex :type Integer) (bFromSweep :type Boolean) (SweepResult :type Hit%20Result%20Structure%20%28by%20ref%29))
  (Utilities|Casting|CastToBP_AI_Bot OtherActor)
  (CallFunction|Detonation))

(event EventBeginPlay
  (Utilities|FlowControl|Delay 3.0)
  (CallFunction|Detonation))

(event Collision|EventActorBeginOverlap
  (params (OtherActor :type Actor%20Object%20Reference)))

(event EventTick
  (params (DeltaSeconds :type Float%20%28single-precision%29)))

(fn ConstructionScript)

(fn Detonation
  (for _array_element (Collision|GetOverlappingActors (Variables|Default|Getexplosion) "/Game/Master/Characters/AI/BP_AI_Bot.BP_AI_Bot_C" :!class /Script/Engine.PrimitiveComponent)
    (bind _asbp_ai_bot (Utilities|Casting|CastToBP_AI_Bot _array_element))
    (Default|BotTakeDamage _asbp_ai_bot (Variables|Default|GetDamage)))
  (Actor|DestroyActor))