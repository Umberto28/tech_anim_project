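; BP_RifleBot is a hitscan rifle for AI bots that damages BP_TACharacter targets.
; On BeginPlay it registers with its parent BP_AI_Bot, fills the magazine and collects all bots as trace-ignored actors.
; HandleShoot gates firing by ammo and a delay, calling FireBullet for a debug-drawn Visibility line trace.
; Reload blocks shooting during a timed refill, with a DoOnce guarding against repeat calls.
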(event Custom|HandleShoot
  (if (Variables|Default|GetCanShoot)
    (if (> (Variables|Default|GetCurrentAmmo) 0)
      (CallFunction|FireBullet)
      (Math|Integer|DecrementInt (Variables|Default|GetCurrentAmmo)
        (:%20%20
          (Variables|Default|SetCanShoot false)
          (Utilities|FlowControl|Delay (Variables|Default|GetFireDelay))
          (Variables|Default|SetCanShoot true))))))

(event Custom|Reload
  (Utilities|FlowControl|DoOnce false :!label _label
    (:Completed
      (Variables|Default|SetCanShoot false)
      (Utilities|FlowControl|Delay (Variables|Default|GetReloadTime))
      (Variables|Default|SetCurrentAmmo (Variables|Default|GetMagSize))
      (Variables|Default|SetCanShoot true)
      (goto _label Reset))))

(event EventBeginPlay
  (bind _asbp_ai_bot (Utilities|Casting|CastToBP_AI_Bot (Actor|GetParentActor)))
  (CallFunction|SetBotValues _asbp_ai_bot))

(fn ConstructionScript)

(fn FireBullet
  (bind _outhit (Collision|LineTraceByChannel (|StartLineTrace) (|EndLineTrace) "TraceTypeQuery1" false (Variables|Default|GetActorsToIgnore) "ForDuration" true "(R=1.000000,G=0.000000,B=0.000000,A=1.000000)" "(R=0.000000,G=1.000000,B=0.000000,A=1.000000)" 5e+01))
  (Utilities|IsValid (.HitActor (Collision|BreakHitResult _outhit))
    (:Is%20Valid
      (bind _asbp_tacharacter (Utilities|Casting|CastToBP_TACharacter (.HitActor (Collision|BreakHitResult _outhit))))
      (Default|TakeDamage _asbp_tacharacter (Math|Conversions|ToFloat(Integer) (Variables|Default|GetDamage))))))

(fn SetBotValues
  (params (Bot :type BP%20AI%20Bot%20Object%20Reference))
  (bind _output_get (Variables|Default|SetRefToChatacter Bot))
  (bind _outactors (Actor|GetAllActorsOfClass "/Game/Master/Characters/AI/BP_AI_Bot.BP_AI_Bot_C"))
  (Variables|Default|SetActorsToIgnore _outactors)
  (Utilities|Array|Add (Variables|Default|GetActorsToIgnore) _output_get)
  (Variables|/Game/Master/Characters/AI/BP_AI_Bot.BP_AI_Bot_C|SetRifle Bot self)
  (Variables|Default|SetCurrentAmmo (Variables|Default|GetMagSize))
  (return))